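; Scene component that makes its owning actor float above surfaces using physics forces.
; On BeginPlay it takes the owner's first primitive component and makes it movable and physics-simulated.
; Each tick it traces downward by the floating height and, on a hit, pushes along the surface normal with a force that fades linearly with distance.
; A hit also applies linear and angular damping, which is never reset.
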(event `self.ReceiveBeginPlay`
  (bind _output_get (set `self.PrimitiveComponent` (`|GetArrayItem` (`Actor.K2_GetComponentsByClass` (`self.GetOwner`) "/Script/Engine.PrimitiveComponent"))))
  (`self.SetMobility` _output_get "Movable")
  (`PrimitiveComponent.SetSimulatePhysics` _output_get true))

(event `self.ReceiveTick`
  (params (DeltaSeconds :type "Float (single-precision)"))
  (bind _returnvalue (`self.K2_GetComponentLocation`))
  (bind (_outhit _returnvalue_2) (`KismetSystemLibrary.LineTraceSingle` _returnvalue (- _returnvalue (`KismetMathLibrary.MakeVector` 0.0 0.0 (`self.FloatingHeight`))) "TraceTypeQuery1" true))
  (if _returnvalue_2
    (bind (_bblockinghit _binitialoverlap _time _distance _location _impactpoint _normal _impactnormal) (`GameplayStatics.BreakHitResult` _outhit))
    (`PrimitiveComponent.AddForce` (`self.PrimitiveComponent`) (* _impactnormal (`KismetMathLibrary.Lerp` (`self.HoverForce`) 0.0 (/ (`KismetMathLibrary.VSize` (- _location (`self.K2_GetComponentLocation`))) (`self.FloatingHeight`)))) "None" false)
    (`PrimitiveComponent.SetLinearDamping` (`self.PrimitiveComponent`) (`self.LinearDamping`))
    (`PrimitiveComponent.SetAngularDamping` (`self.PrimitiveComponent`) (`self.AngularDamping`))))