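; Sliding door actor that moves its mesh between closed and opened transforms, driven by trigger, toggle or crank signals.
; Trigger flips and Toggle sets the open state, if allowed, playing or reversing a timeline rate-scaled to the slide duration; crank updates set the percentage directly.
; The closed-position component is itself the moving door, lerped from its cached transform toward the opened-position component, which shares its mesh.
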(event `self.ReceiveBeginPlay`
  (set `self.Transform When Closed` (`SceneComponent.K2_GetComponentToWorld` (`self.PositionWhenClosed`)) :!label _label)
  (`self.Set Position By Percent` (stale `/Game/Blueprints/Interface/ICrankableObject.CrankWasUpdated` `New Percent Value`) :!label _label_2))

(event `/Game/Blueprints/Interface/ICrankableObject.CrankWasUpdated`
  (params (`New Percent Value` :type "Float (single-precision)"))
  (if (`self.dirty`)
    (set `self.dirty` false)
    (goto _label)
    (else
      (goto _label_2))))

(event `/Game/Blueprints/Interface/ITriggerOrToggle.Trigger`
  (bind _slide (`self.Slide`))
  (if (`self.Allow trigger signals`)
    (set `self.Is door open` (not (`self.Is door open`)))
    (`TimelineComponent.SetPlayRate` _slide (/ (`TimelineComponent.GetTimelineLength` _slide) (`self.How long it takes to slide`)) :!label _label_3)
    (if (`self.Is door open`)
      (bind (_direction _percent) (`Timeline|Slide` :!label _label_4)
        (:`Update`
          (`self.Set Position By Percent` _percent)))
      (else
        (goto _label_4 :!via `Reverse`)))))

(event `/Game/Blueprints/Interface/ITriggerOrToggle.Toggle`
  (params (IsNowOn :type Boolean))
  (if (`self.Allow toggle signals`)
    (set `self.Is door open` IsNowOn)
    (goto _label_3)))

(fn `Set Position By Percent`
  (params (Percent :type "Float (double-precision)"))
  (`SceneComponent.K2_SetWorldTransform` (`self.PositionWhenClosed`) (`KismetMathLibrary.TLerp` (`self.Transform When Closed`) (`SceneComponent.K2_GetComponentToWorld` (`self.PositionWhenOpened`)) Percent) false false))

(fn `UserConstructionScript`
  (`StaticMeshComponent.SetStaticMesh` (`self.PositionWhenClosed`) (`self.Mesh of Door`))
  (`StaticMeshComponent.SetStaticMesh` (`self.PositionWhenOpened`) (`self.Mesh of Door`)))