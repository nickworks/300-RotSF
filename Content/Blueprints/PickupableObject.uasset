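; A physics-driven object actor that the player can pick up, carry, drop, throw or respawn.
; Interacting turns off physics and collision and asks the player character to attach it to their hands.
; Drop and Throw turn both back on, with Throw also setting the mesh's linear velocity.
; Respawn restores the transform saved at BeginPlay and zeroes velocities; the construction script applies a configurable static mesh.
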(event `/Game/Blueprints/Interface/IPlayerCanLookAtAndInteractWith.PlayerWantsToInteract`
  (params (PlayerCharacter :type "/Game/Blueprints/PlayerCharacter Object Reference"))
  (`self.Turn Physics` false)
  (`/Game/Blueprints/PlayerCharacter.AttachObjectToHands` PlayerCharacter self))

(event `/Game/Blueprints/Interface/IPickupObject.Drop`
  (`self.Turn Physics` true))

(event `/Game/Blueprints/Interface/IPickupObject.Throw`
  (params (ThrowDirection :type "Vector Structure"))
  (`self.Turn Physics` true)
  (`PrimitiveComponent.SetPhysicsLinearVelocity` (`self.TheMesh`) ThrowDirection false "None"))

(event `self.ReceiveBeginPlay`
  (set `self.origTransform` (`self.GetTransform`)))

(event `/Game/Blueprints/Interface/ICheckpointActions.Respawn`
  (`self.K2_SetActorTransform` (`self.origTransform`))
  (`PrimitiveComponent.SetPhysicsLinearVelocity` (`self.TheMesh`) (0.0 0.0 0.0) false "None")
  (`PrimitiveComponent.SetPhysicsAngularVelocityInDegrees` (`self.TheMesh`) (`KismetMathLibrary.MakeVector` 0.0) false "None"))

(fn `Turn Physics`
  (params (`Is On?` :type Boolean))
  (`PrimitiveComponent.SetSimulatePhysics` (`self.TheMesh`) `Is On?`)
  (`self.SetActorEnableCollision` `Is On?`)
  (return))

(fn `UserConstructionScript`
  (`StaticMeshComponent.SetStaticMesh` (`self.TheMesh`) (`self.StaticMesh`)))