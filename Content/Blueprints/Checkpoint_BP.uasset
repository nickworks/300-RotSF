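; Checkpoint actor that saves the player's location and can reset a list of level actors.
; When the player character overlaps its Cube, it writes that location to the "checkpoint" save slot, creating the save if needed.
; BeginPlay caches each listed actor's transform and class.
; RespawnActors, not called within this graph, teleports surviving actors back or spawns replacements, then sends RespawnMessage to those implementing the interface.
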(event `self.ReceiveBeginPlay`
  (`self.CacheItems`))

(event `self.Cube.OnComponentBeginOverlap`
  (params (OverlappedComponent :type "PrimitiveComponent Object Reference") (OtherActor :type "Actor Object Reference") (OtherComp :type "PrimitiveComponent Object Reference") (OtherBodyIndex :type Integer) (bFromSweep :type Boolean) (SweepResult :type "HitResult Structure (by ref)"))
  (bind _playerlocation (`self.PlayerLocation`))
  (bind _asplayer_character (cast `/Game/Blueprints/PlayerCharacter` OtherActor))
  (set `self.PlayerLocation` (`self.K2_GetActorLocation` _asplayer_character))
  (bind _returnvalue (`GameplayStatics.DoesSaveGameExist` "checkpoint"))
  (if _returnvalue
    (bind _returnvalue_2 (`GameplayStatics.LoadGameFromSlot` "checkpoint"))
    (bind _assave_game_bp (cast `/Game/Blueprints/SaveGame_BP` _returnvalue_2))
    (set `/Game/Blueprints/SaveGame_BP.PlayerLocationSave` _playerlocation _assave_game_bp)
    (`GameplayStatics.SaveGameToSlot` _assave_game_bp "checkpoint")
    (else
      (bind _returnvalue_3 (`GameplayStatics.CreateSaveGameObject` "/Game/Blueprints/SaveGame_BP.SaveGame_BP_C"))
      (set `/Game/Blueprints/SaveGame_BP.PlayerLocationSave` _playerlocation _returnvalue_3)
      (`GameplayStatics.SaveGameToSlot` _returnvalue_3 "checkpoint"))))

(fn `CacheItems`
  (for _array_element (`self.RespawnActorList`)
    (`KismetArrayLibrary.Array_Add` (`self.LibraryOfActorsToRespawn`) (make `/Game/Blueprints/Structs/CheckpointItem` _array_element (`self.GetTransform` _array_element) (`GameplayStatics.GetObjectClass` _array_element)))))

(fn `RespawnActors`
  (for _array_element (`self.LibraryOfActorsToRespawn`)
    (bind (_actor _location _datatype) (break `/Game/Blueprints/Structs/CheckpointItem` _array_element))
    (`/Engine/EditorBlueprintResources/StandardMacros.IsValid` _actor
      (:`Is Valid`
        (`self.K2_SetActorTransform` _actor _location false true))
      (:`Is Not Valid`
        (bind _returnvalue (`|SpawnActorFromClass` _datatype _location "Undefined" "OverrideRootScale" null null))
        (`|VariableSetRef` _array_element (make `/Game/Blueprints/Structs/CheckpointItem` _returnvalue _location _datatype))))
    (if (`KismetSystemLibrary.DoesImplementInterface` _actor)
      (message `/Game/Blueprints/Interface/ICheckpointActions.Respawn` _actor))))

(fn `UserConstructionScript`)