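; An interactable lever that switches a list of controlled objects on or off, unless it is broken.
; Interaction flips the state, sends it through the ITriggerOrToggle interface to implementing objects, and plays or reverses a timeline that pitches the hinge.
; BeginPlay enters the same path without flipping, so objects and hinge start in sync.
; A broken lever only prints a message and hides its mesh on construction until Fix restores it.
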(event `/Game/Blueprints/Interface/IPlayerCanLookAtAndInteractWith.PlayerWantsToInteract`
  (params (PlayerCharacter :type "/Game/Blueprints/PlayerCharacter Object Reference"))
  (if (`self.IsLeverBroken`)
    (`KismetSystemLibrary.PrintString` "The lever is broken....")
    (else
      (set `self.IsLeverOn` (not (`self.IsLeverOn`)))
      (`self.UpdateControlledObject` :!label _label)
      (if (`self.IsLeverOn`)
        (bind (_direction _hinge_rotation_y) (`Timeline|Throw The Lever!` :!label _label_2)
          (:`Update`
            (`SceneComponent.K2_SetRelativeRotation` (`self.Hinge`) (`KismetMathLibrary.MakeRotator` 0.0 _hinge_rotation_y) false false)))
        (else
          (goto _label_2 :!via `Reverse`))))))

(event `self.ReceiveBeginPlay`
  (goto _label))

(event `InputAction|Interact` :consume false
  (params (Key :type "Key Structure")))

(fn `Fix`
  (set `self.IsLeverBroken` false)
  (`SceneComponent.SetVisibility` (`self.Mesh - Lever`) true false))

(fn `UpdateControlledObject`
  (for _array_element (`self.Controlled Objects`)
    (if (`KismetSystemLibrary.DoesImplementInterface` _array_element "/Game/Blueprints/Interface/ITriggerOrToggle.ITriggerOrToggle_C")
      (message `/Game/Blueprints/Interface/ITriggerOrToggle.Toggle` _array_element (`self.IsLeverOn`)))))

(fn `UserConstructionScript`
  (`SceneComponent.SetVisibility` (`self.Mesh - Lever`) (not (`self.IsLeverBroken`)) false))