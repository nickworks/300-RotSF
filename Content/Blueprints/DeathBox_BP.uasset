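; DeathBox_BP is a kill volume that sends the player into death handling when they overlap its DeathTrigger component.
; On overlap it disables player input, waits briefly and checks for a "checkpoint" save.
; If one exists, it loads and type-checks the save without reading its data, then calls the player's Death and restores input.
; Otherwise it reopens the Sandbox level.
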(event `self.DeathTrigger.OnComponentBeginOverlap`
  (params (OverlappedComponent :type "PrimitiveComponent Object Reference") (OtherActor :type "Actor Object Reference") (OtherComp :type "PrimitiveComponent Object Reference") (OtherBodyIndex :type Integer) (bFromSweep :type Boolean) (SweepResult :type "HitResult Structure (by ref)"))
  (bind _asplayer_character (cast `/Game/Blueprints/PlayerCharacter` OtherActor))
  (`self.DisableInput` _asplayer_character (`GameplayStatics.GetPlayerController` 0))
  (`KismetSystemLibrary.Delay` 0.3)
  (bind _returnvalue (`GameplayStatics.DoesSaveGameExist` "checkpoint"))
  (if _returnvalue
    (bind _returnvalue_2 (`GameplayStatics.LoadGameFromSlot` "checkpoint"))
    (cast `/Game/Blueprints/SaveGame_BP` _returnvalue_2)
    (bind _asplayer_character_2 (cast `/Game/Blueprints/PlayerCharacter` (`GameplayStatics.GetPlayerCharacter` 0)))
    (`/Game/Blueprints/PlayerCharacter.Death` _asplayer_character_2)
    (`self.EnableInput` _asplayer_character_2 (`GameplayStatics.GetPlayerController` 0))
    (else
      (`GameplayStatics.OpenLevel` (`self.Sandbox`)))))

(fn `UserConstructionScript`)