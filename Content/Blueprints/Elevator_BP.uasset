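; Elevator Blueprint that moves its Elevator component along a spline, driven by crank updates or by trigger and toggle events.
; One timeline combines travel distance with the crank's percent value to place the elevator on the spline.
; A second timeline plays or reverses at a rate derived from the travel time.
; AllowTriggersToToggleToo selects whether Trigger flips the open state or Toggle sets it.
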(event `self.ReceiveBeginPlay`
  ;[1 1 1] Crank Controlled Elevator
  (bind (_direction _traveldistance) (`Timeline|MoveElevator` :!via `SetNewTime` :!label _label)
    (:`Update`
      (`SceneComponent.K2_SetWorldLocation` (`self.Elevator`) (`SplineComponent.GetLocationAtDistanceAlongSpline` (`self.Spline`) (* (* _traveldistance (`SplineComponent.GetSplineLength` (`self.Spline`))) (stale `/Game/Blueprints/Interface/ICrankableObject.CrankWasUpdated` `New Percent Value`)) "World") false false))))

(event `/Game/Blueprints/Interface/ICrankableObject.CrankWasUpdated`
  (params (`New Percent Value` :type "Float (single-precision)"))
  ;[1 1 1] Crank Controlled Elevator
  (goto _label))

(event `/Game/Blueprints/Interface/ITriggerOrToggle.Trigger`
  (if (`self.Allow triggers to toggle too`)
    (set `self.IsOpen` (not (`self.IsOpen`)))
    (`TimelineComponent.SetPlayRate` (`self.MoveElevatorWithTriggerOrToggle`) (/ (`TimelineComponent.GetTimelineLength` (`self.MoveElevatorWithTriggerOrToggle`)) (`self.TravelTimeTriggerOrToggle`)) :!label _label_2)
    (if (`self.IsOpen`)
      (bind (_direction _traveldistance) (`Timeline|MoveElevatorWithTriggerOrToggle` :!label _label_3)
        (:`Update`
          (`SceneComponent.K2_SetWorldLocation` (`self.Elevator`) (`SplineComponent.GetLocationAtDistanceAlongSpline` (`self.Spline`) (* _traveldistance (`SplineComponent.GetSplineLength` (`self.Spline`))) "World") false false)))
      (else
        (goto _label_3 :!via `Reverse`)))))

(event `/Game/Blueprints/Interface/ITriggerOrToggle.Toggle`
  (params (IsNowOn :type Boolean))
  (if (not (`self.Allow triggers to toggle too`))
    (set `self.IsOpen` IsNowOn)
    (goto _label_2)))

(fn `UserConstructionScript`)