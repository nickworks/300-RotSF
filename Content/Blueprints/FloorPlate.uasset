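; FloorPlate is a one-shot pressure plate actor that switches linked objects when hit.
; On Hit it sets IsPressed, drops 20 units and disables its collision; the PlayerCharacter cast is disconnected, so any actor triggers it.
; UpdateControlledObjects then loops over ControlledObjects and sends an interface ToggleMessage with false to each that implements the interface.
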(event `self.ReceiveHit`
  (params (MyComp :type "PrimitiveComponent Object Reference") (Other :type "Actor Object Reference") (OtherComp :type "PrimitiveComponent Object Reference") (bSelfMoved :type Boolean) (HitLocation :type "Vector Structure") (HitNormal :type "Vector Structure") (NormalImpulse :type "Vector Structure") (Hit :type "HitResult Structure (by ref)"))
  (if true
    (set `self.IsPressed` true)
    (`self.K2_SetActorLocation` (+ (`self.K2_GetActorLocation`) (0.0 0.0 -20.0)))
    (`self.SetActorEnableCollision` false)
    (`self.UpdateControlledObjects`)))

(fn `UpdateControlledObjects`
  (for _array_element (`self.ControlledObjects`)
    (if (`KismetSystemLibrary.DoesImplementInterface` _array_element)
      (message `/Game/Blueprints/Interface/ITriggerOrToggle.Toggle` _array_element false))))

(fn `UserConstructionScript`)