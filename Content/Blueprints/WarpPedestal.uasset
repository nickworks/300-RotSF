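; Warp pedestal that toggles a floating 3D map widget when the player interacts, unless it is broken.
; Its overlap sphere enables input so Fire clicks through WidgetInteraction, and closes the map when the player leaves.
; Tick turns the map toward the camera and eases its scale, hiding it once shrunk to zero.
; Broken pedestals hide their Sphere until Fix receives a pickupable flagged to repair them.
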(event `self.ReceiveBeginPlay`)

(event `self.ReceiveTick`
  (params (DeltaSeconds :type "Float (single-precision)"))
  (`self.RotateMapTowardsPlayer`)
  (`self.Scale Map`))

(event `InputAction|Fire` :consume false
  (params (Key :type "Key Structure"))
  (bind _widgetinteraction (`self.WidgetInteraction`))
  (:`Pressed`
    (`WidgetInteractionComponent.PressPointerKey` _widgetinteraction "LeftMouseButton"))
  (:`Released`
    (`WidgetInteractionComponent.ReleasePointerKey` _widgetinteraction "LeftMouseButton")))

(event `self.Sphere1.OnComponentBeginOverlap`
  (params (OverlappedComponent :type "PrimitiveComponent Object Reference") (OtherActor :type "Actor Object Reference") (OtherComp :type "PrimitiveComponent Object Reference") (OtherBodyIndex :type Integer) (bFromSweep :type Boolean) (SweepResult :type "HitResult Structure (by ref)"))
  (cast `/Game/Blueprints/PlayerCharacter` OtherActor)
  (`self.EnableInput` (`GameplayStatics.GetPlayerController` 0)))

(event `self.Sphere1.OnComponentEndOverlap`
  (params (OverlappedComponent :type "PrimitiveComponent Object Reference") (OtherActor :type "Actor Object Reference") (OtherComp :type "PrimitiveComponent Object Reference") (OtherBodyIndex :type Integer))
  (cast `/Game/Blueprints/PlayerCharacter` OtherActor)
  (`self.DisableInput` (`GameplayStatics.GetPlayerController` 0))
  (`self.ToggleShowMap` false))

(event `/Game/Blueprints/Interface/IPlayerCanLookAtAndInteractWith.PlayerWantsToInteract`
  (params (PlayerCharacter :type "/Game/Blueprints/PlayerCharacter Object Reference"))
  (if (not (`self.Is broken?`))
    (`self.ToggleShowMap` (not (`self.Is showing map`)))))

(fn `Fix`
  (params (`Currently held item` :type "Actor Object Reference"))
  (returns (`Is It Fixed?` :type Boolean))
  (bind _aspickupable_object (cast `/Game/Blueprints/PickupableObject` `Currently held item`)
    (:`then`
      (if (`/Game/Blueprints/PickupableObject.Fixes warp pedestals` _aspickupable_object)
        (if (`self.Is broken?`)
          (set `self.Is broken?` false)
          (`SceneComponent.SetVisibility` (`self.Sphere`) true false)
          (return true)
          (else
            _))))
    (:`CastFailed`
      _))
  (return false))

(fn `RotateMapTowardsPlayer`
  (if (`self.Is showing map`)
    (`SceneComponent.K2_SetWorldRotation` (`self.Widget`) (`KismetMathLibrary.FindLookAtRotation` (`SceneComponent.K2_GetComponentLocation` (`self.Widget`)) (`self.GetActorEyesViewPoint` (`GameplayStatics.GetPlayerCameraManager` 0))) false false)))

(fn `Scale Map`
  (bind _widget (`self.Widget`))
  (bind _relativescale3d_x (`KismetMathLibrary.BreakVector` (`SceneComponent.RelativeScale3D` _widget)))
  (bind _returnvalue (+ _relativescale3d_x (* (- (select `bool` (`self.Is showing map`) :`false` -0.1 :`true` 0.6 :!type "Float (single-precision)") _relativescale3d_x) 0.1)))
  (if (`SceneComponent.IsVisible` (`self.Widget`))
    (if (<= _returnvalue 0.0)
      (`SceneComponent.SetVisibility` (`self.Widget`) false false)
      (else
        (`SceneComponent.SetRelativeScale3D` _widget (`KismetMathLibrary.Conv_DoubleToVector` _returnvalue))))))

(fn `ToggleShowMap`
  (params (`Is map on?` :type Boolean))
  (bind _output_get (set `self.Is showing map` `Is map on?`))
  (`ActorComponent.SetActive` (`self.WidgetInteraction`) _output_get false)
  (if (`self.Is showing map`)
    (`SceneComponent.SetVisibility` (`self.Widget`) true false)))

(fn `UserConstructionScript`
  (`SceneComponent.SetVisibility` (`self.Sphere`) (not (`self.Is broken?`)) false))